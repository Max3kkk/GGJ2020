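; First-person player character handling movement, timer-driven sprint stamina, a three-slot inventory and task interactions.
; A trigger overlap caches the object's type, so Interact runs a wrench-gated slider QTE, button-mash blockage, entry UI or item-slot swap.
; Inventory keys pick two slots to craft "BATA" from batteries; modal UIs freeze time dilation and lock mouse look.
; Tick shows the WIN widget once the generator-repair, battery-craft and trash-clear flags are set.
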(event OnComponentBeginOverlap(Trigger)
  (params (OverlappedComponent :type Primitive%20Component%20Object%20Reference) (OtherActor :type Actor%20Object%20Reference) (OtherComp :type Primitive%20Component%20Object%20Reference) (OtherBodyIndex :type Integer) (bFromSweep :type Boolean) (SweepResult :type Hit%20Result%20Structure%20%28by%20ref%29))
  ;[1 1 1] Триггер
  (bind _asbase_class (Utilities|Casting|CastToBaseClass OtherActor))
  (Variables|Default|SetObjType (Variables|/Game/Scripts/Models/BaseClass.BaseClass_C|GetType _asbase_class))
  (Variables|Default|SetObj _asbase_class)
  (Development|PrintString (Utilities|String|EnumtoString (Variables|/Game/Scripts/Models/BaseClass.BaseClass_C|GetType _asbase_class))))

(event OnComponentEndOverlap(Trigger)
  (params (OverlappedComponent :type Primitive%20Component%20Object%20Reference) (OtherActor :type Actor%20Object%20Reference) (OtherComp :type Primitive%20Component%20Object%20Reference) (OtherBodyIndex :type Integer))
  ;[1 1 1] Ненужное - нужное говно
  (Variables|Default|SetObjType "NewEnumerator0"))

(event Custom|DecreaseStamina
  ;[1 1 1] Передвижение
  (bind _output_get (Variables|Default|SetCurrStamina (- (Variables|Default|GetCurrStamina) 1.0)))
  (if (<= _output_get 0.0)
    (Utilities|Time|ClearandInvalidateTimerbyHandle (stale Input|ActionEvents|InputActionSprint _returnvalue))
    (Variables|/Script/Engine.CharacterMovementComponent|SetMaxWalkSpeed (Variables|Character|GetCharacterMovement) (Variables|Default|GetWalkSpeed))
    (bind _returnvalue (Utilities|Time|SetTimerbyEvent (delegate Custom|IncreaseStamina) 0.05 true))))

(event Custom|IncreaseStamina
  ;[1 1 1] Передвижение
  (bind _output_get (Variables|Default|SetCurrStamina (+ (Variables|Default|GetCurrStamina) 1.0)))
  (if (>= _output_get (Variables|Default|GetMaxStamina))
    (Utilities|Time|ClearandInvalidateTimerbyHandle (stale Input|ActionEvents|InputActionSprint _returnvalue_2))
    (Utilities|Time|ClearandInvalidateTimerbyHandle (stale Custom|DecreaseStamina _returnvalue))))

(event EventBeginPlay
  ;[1 1 1] Начало
  (Variables|/Script/Engine.CharacterMovementComponent|SetMaxWalkSpeed (Variables|Character|GetCharacterMovement) (Variables|Default|GetWalkSpeed))
  (bind _returnvalue (UserInterface|CreateWidget "/Game/UI/Center.Center_C"))
  (UserInterface|Viewport|AddtoViewport _returnvalue 0)
  (Variables|Default|SetCenter _returnvalue)
  (bind _returnvalue_2 (UserInterface|CreateWidget "/Game/UI/Menu.Menu_C"))
  (UserInterface|Viewport|AddtoViewport _returnvalue_2 0)
  (Variables|Default|SetPauseUI _returnvalue_2)
  (bind _returnvalue_3 (UserInterface|CreateWidget "/Game/UI/TimerAndTasks.TimerAndTasks_C"))
  (UserInterface|Viewport|AddtoViewport _returnvalue_3 0))

(event EventTick
  (params (DeltaSeconds :type Float%20%28single-precision%29))
  (if (and (and (Variables|Default|GetRepairGen) (Variables|Default|GetCraftBata)) (Variables|Default|GetClearTrash))
    (bind _returnvalue (UserInterface|CreateWidget "/Game/UI/WIN.WIN_C"))
    (UserInterface|Viewport|AddtoViewport _returnvalue 0)))

(event Input|ActionEvents|InputActionSprint
  (params (Key :type Key%20Structure))
  (bind _charactermovement (Variables|Character|GetCharacterMovement))
  ;[1 1 1] Передвижение
  (:Pressed
    (Variables|/Script/Engine.CharacterMovementComponent|SetMaxWalkSpeed _charactermovement (Variables|Default|GetRunSpeed))
    (bind _returnvalue (Utilities|Time|SetTimerbyEvent (delegate Custom|DecreaseStamina) 0.05 true))
    (Utilities|Time|ClearandInvalidateTimerbyHandle (stale _returnvalue_2))
    (Utilities|Time|ClearandInvalidateTimerbyHandle (stale Custom|DecreaseStamina _returnvalue)))
  (:Released
    (Variables|/Script/Engine.CharacterMovementComponent|SetMaxWalkSpeed _charactermovement (Variables|Default|GetWalkSpeed))
    (bind _returnvalue_2 (Utilities|Time|SetTimerbyEvent (delegate Custom|IncreaseStamina) 0.05 true))
    (Utilities|Time|ClearandInvalidateTimerbyHandle _returnvalue)))

(event Input|ActionEvents|InputActionInventory
  (params (Key :type Key%20Structure))
  ;[1 1 1] Открытие инвентаря
  (:Pressed
    (if (Variables|Default|GetInventoryVisible)
      (Variables|Default|SetInventoryVisible false)
      (Variables|/Script/Engine.PlayerController|SetbShowMouseCursor (Game|GetPlayerController 0) false)
      (Utilities|Time|SetGlobalTimeDilation 1.0)
      (Variables|Default|SetLockMouse false)
      (Widget|RemovefromParent (Variables|Default|GetInventory))
      (Variables|Default|SetFirst 0)
      (Variables|Default|SetSecond 0)
      (Variables|Default|SetNumCraft 0)
      (else
        (bind _returnvalue (UserInterface|CreateWidget "/Game/UI/Inventory.Inventory_C"))
        (UserInterface|Viewport|AddtoViewport _returnvalue 0)
        (bind _output_get (Variables|Default|SetInventory _returnvalue))
        (Variables|Default|SetInventoryVisible true)
        (Default|Override _output_get (Variables|Default|GetSlot%201) 1)
        (Default|Override _output_get (Variables|Default|GetSlot%202) 2)
        (Default|Override _output_get (Variables|Default|GetSlot%203) 3)
        (Variables|/Script/Engine.PlayerController|SetbShowMouseCursor (Game|GetPlayerController 0) true)
        (Utilities|Time|SetGlobalTimeDilation 0.0)
        (Variables|Default|SetLockMouse true)))))

(event Input|ActionEvents|InputActionJumping
  (params (Key :type Key%20Structure))
  ;[1 1 1] Передвижение
  (:Pressed
    (Character|Jump)))

(event Input|ActionEvents|InputActionCraft
  (params (Key :type Key%20Structure))
  (bind _item (Variables|Default|GetItem))
  (bind _item_2 (Variables|Default|GetItem))
  (:Pressed
    (if (Variables|Default|GetInventoryVisible)
      (switch int (Variables|Default|GetFirst)
        (:1
          (Variables|Default|SetF (Variables|Default|GetSlot%201)))
        (:2
          (Variables|Default|SetF (Variables|Default|GetSlot%202)))
        (:3
          (Variables|Default|SetF (Variables|Default|GetSlot%203))))
      (switch int (Variables|Default|GetSecond)
        (:1
          (Variables|Default|SetS (Variables|Default|GetSlot%201)))
        (:2
          (Variables|Default|SetS (Variables|Default|GetSlot%202)))
        (:3
          (Variables|Default|SetS (Variables|Default|GetSlot%203))))
      (if (and (Utilities|Enum|Equal(Enum) (.name (.item (Variables|Default|GetS))) (.name (.item (Variables|Default|GetF)))) (Utilities|Enum|Equal(Enum) (.name (.item (Variables|Default|GetF))) "Batarry"))
        (switch int (Variables|Default|GetFirst)
          (:1
            (Variables|Default|SetSlot%201 (Utilities|Struct|MakeSlotStructure (Utilities|Struct|MakeItemStructure _item "/Game/Scripts/Player/Fon.Fon" "None" 0))))
          (:2
            (Variables|Default|SetSlot%202 (Utilities|Struct|MakeSlotStructure (Utilities|Struct|MakeItemStructure _item "/Game/Scripts/Player/Fon.Fon" "None" 0))))
          (:3
            (Variables|Default|SetSlot%203 (Utilities|Struct|MakeSlotStructure (Utilities|Struct|MakeItemStructure _item "/Game/Scripts/Player/Fon.Fon" "None" 0)))))
        (switch int (Variables|Default|GetSecond)
          (:1
            (Variables|Default|SetSlot%201 (Utilities|Struct|MakeSlotStructure (Utilities|Struct|MakeItemStructure _item_2 "/Game/Scripts/Player/Fon.Fon" "None" 0))))
          (:2
            (Variables|Default|SetSlot%202 (Utilities|Struct|MakeSlotStructure (Utilities|Struct|MakeItemStructure _item_2 "/Game/Scripts/Player/Fon.Fon" "None" 0))))
          (:3
            (Variables|Default|SetSlot%203 (Utilities|Struct|MakeSlotStructure (Utilities|Struct|MakeItemStructure _item_2 "/Game/Scripts/Player/Fon.Fon" "None" 0)))))
        (switch int (Variables|Default|GetFirst)
          (:1
            (Variables|Default|SetSlot%201 (Utilities|Struct|MakeSlotStructure (Utilities|Struct|MakeItemStructure "BATA" 0 "None" 0))))
          (:2
            (Variables|Default|SetSlot%202 (Utilities|Struct|MakeSlotStructure (Utilities|Struct|MakeItemStructure "BATA" 0 "None" 0))))
          (:3
            (Variables|Default|SetSlot%203 (Utilities|Struct|MakeSlotStructure (Utilities|Struct|MakeItemStructure "BATA" 0 "None" 0)))))
        (Widget|RemovefromParent (Variables|Default|GetInventory))
        (Variables|Default|SetInventoryVisible false)
        (Variables|/Script/Engine.PlayerController|SetbShowMouseCursor (Game|GetPlayerController 0) false)
        (Utilities|Time|SetGlobalTimeDilation 1.0)
        (Variables|Default|SetLockMouse false)
        (Variables|Default|SetCraftBata true)
        (else
          (Variables|Default|SetFirst 0)
          (Variables|Default|SetSecond 0)
          (Variables|Default|SetNumCraft 0))))))

(event Input|ActionEvents|InputActionInteract
  (params (Key :type Key%20Structure))
  (bind _item (Variables|Default|GetItem))
  ;[1 1 1] Инвентарь и QTE
  (:Pressed
    (if (Math|Boolean|NotEqual(Boolean) (Variables|Default|GetIsActive) true)
      (switch Utilities|FlowControl|Switch|SwitchonPressE (Variables|Default|GetObjType)
        (:NewEnumerator1
          (bind (_answer _pos) (CallFunction|CheckInventory))
          (Variables|Default|SetCan _answer)
          (Variables|Default|SetCanPos _pos)
          (if _answer
            (bind _returnvalue (UserInterface|CreateWidget "/Game/UI/UI_QTE.UI_QTE_C"))
            (UserInterface|Viewport|AddtoViewport _returnvalue 0)
            (Variables|Default|SetUIQte _returnvalue)
            (Utilities|Time|SetGlobalTimeDilation 0.0)
            (Variables|Default|SetIsActive true)
            (Variables|Default|SetLockMouse true)
            (Widget|SetVisibility (Variables|Default|GetCenter) "Hidden" :!label _label)))
        (:NewEnumerator2
          (bind _returnvalue_2 (UserInterface|CreateWidget "/Game/UI/UI_Blockage.UI_Blockage_C"))
          (UserInterface|Viewport|AddtoViewport _returnvalue_2 0)
          (bind _output_get (Variables|Default|SetUIBlock _returnvalue_2))
          (Utilities|Time|SetGlobalTimeDilation 0.0)
          (Variables|Default|SetIsActive true)
          (Variables|Default|SetLockMouse true)
          (Variables|/Game/UI/UI_Blockage.UI_Blockage_C|SetObj _output_get (Variables|Default|GetObj))
          (goto _label))
        (:NewEnumerator3
          (Variables|/Script/Engine.PlayerController|SetbShowMouseCursor (Game|GetPlayerController 0) true)
          (bind _returnvalue_3 (UserInterface|CreateWidget "/Game/UI/UI_Enter.UI_Enter_C"))
          (UserInterface|Viewport|AddtoViewport _returnvalue_3 0)
          (bind _output_get_2 (Variables|Default|SetUIEnter _returnvalue_3))
          (Utilities|Time|SetGlobalTimeDilation 0.0)
          (Variables|Default|SetIsActive true)
          (Variables|/Game/UI/UI_Enter.UI_Enter_C|SetObj _output_get_2 (Variables|Default|GetObj))
          (Variables|Default|SetLockMouse true)
          (goto _label))
        (:NewEnumerator5
          (if (Utilities|Enum|Equal(Enum) (Variables|Default|GetItem) (.name (.item (Variables|Default|GetSlot%201))))
            (bind _asbc_insert (Utilities|Casting|CastToBC_Insert (Variables|Default|GetObj)))
            (Variables|Default|SetSlot%201 (Utilities|Struct|MakeSlotStructure (Utilities|Struct|MakeItemStructure (.name (Variables|/Game/Scripts/Models/Insert/BC_Insert.BC_Insert_C|GetItemStructure _asbc_insert)) (.thumbnail (Variables|/Game/Scripts/Models/Insert/BC_Insert.BC_Insert_C|GetItemStructure _asbc_insert)) "None" 0)))
            (Class|InteractInterface|Interact(Message) (Variables|Default|GetObj) (Variables|Default|GetObj))
            (elif (Utilities|Enum|Equal(Enum) (Variables|Default|GetItem) (.name (.item (Variables|Default|GetSlot%202))))
              (bind _asbc_insert_2 (Utilities|Casting|CastToBC_Insert (Variables|Default|GetObj)))
              (Variables|Default|SetSlot%202 (Utilities|Struct|MakeSlotStructure (Utilities|Struct|MakeItemStructure (.name (Variables|/Game/Scripts/Models/Insert/BC_Insert.BC_Insert_C|GetItemStructure _asbc_insert_2)) (.thumbnail (Variables|/Game/Scripts/Models/Insert/BC_Insert.BC_Insert_C|GetItemStructure _asbc_insert_2)) "None" 0)))
              (Class|InteractInterface|Interact(Message) (Variables|Default|GetObj) (Variables|Default|GetObj))
              (elif (Utilities|Enum|Equal(Enum) (Variables|Default|GetItem) (.name (.item (Variables|Default|GetSlot%203))))
                (bind _asbc_insert_3 (Utilities|Casting|CastToBC_Insert (Variables|Default|GetObj)))
                (Variables|Default|SetSlot%203 (Utilities|Struct|MakeSlotStructure (Utilities|Struct|MakeItemStructure (.name (Variables|/Game/Scripts/Models/Insert/BC_Insert.BC_Insert_C|GetItemStructure _asbc_insert_3)) (.thumbnail (Variables|/Game/Scripts/Models/Insert/BC_Insert.BC_Insert_C|GetItemStructure _asbc_insert_3)) "None" 0)))
                (Class|InteractInterface|Interact(Message) (Variables|Default|GetObj) (Variables|Default|GetObj))
                (else
                  (Development|PrintString "Пошел в пезду")))))))
      (else
        (switch Utilities|FlowControl|Switch|SwitchonPressE (Variables|Default|GetObjType)
          (:NewEnumerator1
            (if (and (>= (Class|Slider|GetValue (Variables|/Game/UI/UI_QTE.UI_QTE_C|GetSlider_91 (Variables|Default|GetUIQte))) 0.48) (<= (Class|Slider|GetValue (Variables|/Game/UI/UI_QTE.UI_QTE_C|GetSlider_91 (Variables|Default|GetUIQte))) 0.55))
              (switch int (Variables|Default|GetCanPos)
                (:1
                  (Variables|Default|SetSlot%201 (Utilities|Struct|MakeSlotStructure (Utilities|Struct|MakeItemStructure _item "/Game/Scripts/Player/Fon.Fon" "None" 0))))
                (:2
                  (Variables|Default|SetSlot%202 (Utilities|Struct|MakeSlotStructure (Utilities|Struct|MakeItemStructure _item "/Game/Scripts/Player/Fon.Fon" "None" 0))))
                (:3
                  (Variables|Default|SetSlot%203 (Utilities|Struct|MakeSlotStructure (Utilities|Struct|MakeItemStructure _item "/Game/Scripts/Player/Fon.Fon" "None" 0)))))
              (Variables|Default|SetRepairGen true))
            (Variables|Default|SetIsActive false)
            (Utilities|Time|SetGlobalTimeDilation 1.0)
            (Variables|Default|SetLockMouse false)
            (Widget|RemovefromParent (Variables|Default|GetUIQte))
            (Widget|SetVisibility (Variables|Default|GetCenter) "Visible"))
          (:NewEnumerator2
            (Class|Slider|SetValue (Variables|/Game/UI/UI_Blockage.UI_Blockage_C|GetSlider_44 (Variables|Default|GetUIBlock)) (+ (Class|Slider|GetValue (Variables|/Game/UI/UI_Blockage.UI_Blockage_C|GetSlider_44 (Variables|Default|GetUIBlock))) 0.108))))))))

(event Input|ActionEvents|InputActionPause
  (params (Key :type Key%20Structure))
  (:Pressed
    (if (Variables|Default|GetisPause)
      (Widget|RemovefromParent (Variables|Default|GetPauseUI))
      (Variables|Default|SetisPause false)
      (else
        (bind _returnvalue (UserInterface|CreateWidget "/Game/UI/Menu.Menu_C"))
        (UserInterface|Viewport|AddtoViewport _returnvalue 0)
        (Variables|Default|SetPauseUI _returnvalue)
        (Variables|Default|SetisPause true)))))

(event Input|AxisEvents|InputAxisMoveForward
  (params (AxisValue :type Float%20%28single-precision%29))
  ;[1 1 1] Движение мышки и передвижение
  (Pawn|Input|AddMovementInput (Transformation|GetActorForwardVector) AxisValue false))

(event Input|AxisEvents|InputAxisMoveRight
  (params (AxisValue :type Float%20%28single-precision%29))
  ;[1 1 1] Движение мышки и передвижение
  (Pawn|Input|AddMovementInput (Transformation|GetActorRightVector) AxisValue false))

(event Input|AxisEvents|InputAxisLookHorizontal
  (params (AxisValue :type Float%20%28single-precision%29))
  ;[1 1 1] Движение мышки и передвижение
  (if (not (Variables|Default|GetLockMouse))
    (Pawn|Input|AddControllerYawInput AxisValue)))

(event Input|AxisEvents|InputAxisLookVertical
  (params (AxisValue :type Float%20%28single-precision%29))
  ;[1 1 1] Движение мышки и передвижение
  (if (not (Variables|Default|GetLockMouse))
    (Pawn|Input|AddControllerPitchInput AxisValue)))

(event Input|KeyboardEvents|1
  (params (Key :type Key%20Structure))
  (:Pressed
    (if (Variables|Default|GetInventoryVisible)
      (if (< (Variables|Default|GetNumCraft) 2)
        (if (not (Variables|Default|GetUsedFirst))
          (if (Utilities|Enum|NotEqual(Enum) (.name (.item (Variables|Default|GetSlot%201))) (Variables|Default|GetItem))
            (Variables|Default|SetUsedFirst true)
            (if (== (Variables|Default|GetNumCraft) 0)
              (Variables|Default|SetFirst 1)
              (bind _result (Math|Integer|IncrementInt (Variables|Default|GetNumCraft))
                (:%20%20
                  (Variables|Default|SetNumCraft _result)))
              (elif (== (Variables|Default|GetNumCraft) 1)
                (Variables|Default|SetSecond 1)
                (bind _result_2 (Math|Integer|IncrementInt (Variables|Default|GetNumCraft))
                  (:%20%20
                    (Variables|Default|SetNumCraft _result_2)))))))))))

(event Input|KeyboardEvents|2
  (params (Key :type Key%20Structure))
  (:Pressed
    (if (Variables|Default|GetInventoryVisible)
      (if (< (Variables|Default|GetNumCraft) 2)
        (if (not (Variables|Default|GetUsedSecond))
          (if (Utilities|Enum|NotEqual(Enum) (Variables|Default|GetItem) (.name (.item (Variables|Default|GetSlot%202))))
            (Variables|Default|SetUsedSecond true)
            (if (== (Variables|Default|GetNumCraft) 0)
              (Variables|Default|SetFirst 2)
              (bind _result (Math|Integer|IncrementInt (Variables|Default|GetNumCraft))
                (:%20%20
                  (Variables|Default|SetNumCraft _result)))
              (elif (== (Variables|Default|GetNumCraft) 1)
                (Variables|Default|SetSecond 2)
                (bind _result_2 (Math|Integer|IncrementInt (Variables|Default|GetNumCraft))
                  (:%20%20
                    (Variables|Default|SetNumCraft _result_2)))))))))))

(event Input|KeyboardEvents|3
  (params (Key :type Key%20Structure))
  (:Pressed
    (if (Variables|Default|GetInventoryVisible)
      (if (< (Variables|Default|GetNumCraft) 2)
        (if (not (Variables|Default|GetUsedThird))
          (if (Utilities|Enum|NotEqual(Enum) (.name (.item (Variables|Default|GetSlot%203))) (Variables|Default|GetItem))
            (Variables|Default|SetUsedThird true)
            (if (== (Variables|Default|GetNumCraft) 0)
              (Variables|Default|SetFirst 3)
              (bind _result (Math|Integer|IncrementInt (Variables|Default|GetNumCraft))
                (:%20%20
                  (Variables|Default|SetNumCraft _result)))
              (elif (== (Variables|Default|GetNumCraft) 1)
                (Variables|Default|SetSecond 3)
                (bind _result_2 (Math|Integer|IncrementInt (Variables|Default|GetNumCraft))
                  (:%20%20
                    (Variables|Default|SetNumCraft _result_2)))))))))))

(fn ConstructionScript)

(fn CheckInventory
  (if (Utilities|Enum|Equal(Enum) (.name (.item (Variables|Default|GetSlot%201))) "Wrench")
    (LocalVariables|SetCheck true)
    (LocalVariables|SetPosition 1)
    (elif (Utilities|Enum|Equal(Enum) (.name (.item (Variables|Default|GetSlot%202))) "Wrench")
      (LocalVariables|SetCheck true)
      (LocalVariables|SetPosition 2)
      (elif (Utilities|Enum|Equal(Enum) (.name (.item (Variables|Default|GetSlot%203))) "Wrench")
        (LocalVariables|SetCheck true)
        (LocalVariables|SetPosition 1)
        (else
          (LocalVariables|SetCheck false)))))
  (return (LocalVariables|GetCheck) (LocalVariables|GetPosition)))